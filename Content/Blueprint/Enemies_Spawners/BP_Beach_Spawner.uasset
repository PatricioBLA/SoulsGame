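; BP_Beach_Spawner is a one-shot trigger that spawns two AI enemies when something overlaps its Box, with no check on the overlapping actor.
; After a short delay, a Niagara smoke explosion plays at each of the two Billboard components, which serve as spawn points.
; Shortly afterwards, a BP_Enemy running BT_Enemy spawns at each point with a fixed rotation.
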(event OnComponentBeginOverlap(Box)
  (params (OverlappedComponent :type Primitive%20Component%20Object%20Reference) (OtherActor :type Actor%20Object%20Reference) (OtherComp :type Primitive%20Component%20Object%20Reference) (OtherBodyIndex :type Integer) (bFromSweep :type Boolean) (SweepResult :type Hit%20Result%20Structure%20%28by%20ref%29))
  (bind _billboard (Variables|Default|GetBillboard))
  (bind _billboard1 (Variables|Default|GetBillboard1))
  (bind _returnvalue (Transformation|GetWorldLocation _billboard1))
  (bind _returnvalue_2 (Transformation|GetWorldLocation _billboard))
  (Utilities|FlowControl|DoOnce false
    (:Completed
      (Utilities|FlowControl|Delay 1.0)
      (Niagara|SpawnSystematLocation "/Game/VFX/NG_Smoke_Explotion.NG_Smoke_Explotion" _returnvalue)
      (Niagara|SpawnSystematLocation "/Game/VFX/NG_Smoke_Explotion.NG_Smoke_Explotion" _returnvalue_2)
      (Utilities|FlowControl|Delay 0.5)
      (Utilities|FlowControl|Sequence
        (:then_0
          (AI|SpawnAIFromClass "/Game/AI/BP_Enemy.BP_Enemy_C" "/Game/AI/BT_Enemy.BT_Enemy" _returnvalue_2 "0.000000,-90.000000,0.000000" false 0))
        (:then_1
          (AI|SpawnAIFromClass "/Game/AI/BP_Enemy.BP_Enemy_C" "/Game/AI/BT_Enemy.BT_Enemy" _returnvalue "0.000000,-90.000000,0.000000" false 0))))))

(fn ConstructionScript)
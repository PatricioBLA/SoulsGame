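; Player combat component for BP_ThirdPersonCharacter_P1, handling target lock, sword combos and dodging, with stamina drawn from BPCStats.
; Lock-on sphere-traces ahead of the camera, attaches a marker actor and steers control rotation toward the target each tick.
; Montage notifies continue or stop combos based on buffered input, while timer-driven sphere traces between sword arrows apply throttled damage.
; Dodge montages follow the WASD key while locked on, otherwise forward.
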(event Custom|Begin%20Damage%20Trace
  ;[0 0.009134 0.06125] Sword Traces
  (bind _returnvalue (Utilities|Time|SetTimerbyEvent (delegate Custom|Damage%20Trace) 0.01 true)))

(event Custom|Damage%20Trace
  (bind _player_bp (Variables|Default|GetPlayer%20BP))
  ;[0 0.009134 0.06125] Sword Traces
  (bind (_outhit _returnvalue) (Collision|SphereTraceForObjects (Transformation|GetWorldLocation (Variables|/Game/ThirdPerson/Blueprints/BP_ThirdPersonCharacter_P1.BP_ThirdPersonCharacter_P1_C|GetStart%20sword%20trace%20arrow _player_bp)) (Transformation|GetWorldLocation (Variables|/Game/ThirdPerson/Blueprints/BP_ThirdPersonCharacter_P1.BP_ThirdPersonCharacter_P1_C|GetEnd%20sword%20trace%20arrow _player_bp)) 25.0 (Utilities|Array|MakeArray "ObjectTypeQuery3") false 0 "ForOneFrame"))
  (if _returnvalue
    (Utilities|FlowControl|DoOnce false :!label _label
      (:Completed
        (Game|Damage|ApplyDamage (.HitActor (Collision|BreakHitResult _outhit)) (Variables|Default|GetSword%20Damage) 0 0)
        (Utilities|FlowControl|Delay 0.3)
        (goto _label Reset)))))

(event Custom|End%20Damage%20Trace
  ;[0 0.009134 0.06125] Sword Traces
  (if (Utilities|Time|IsValidTimerHandle (stale Custom|Begin%20Damage%20Trace _returnvalue))
    (Utilities|Time|ClearandInvalidateTimerbyHandle (stale Custom|Begin%20Damage%20Trace _returnvalue))))

(event Input|EnhancedActionEvents|EnhancedInputActionIA_Lock
  (params (ActionValue :type Boolean) (ElapsedSeconds :type Float%20%28double-precision%29) (TriggeredSeconds :type Float%20%28double-precision%29) (InputAction :type Input%20Action%20Object%20Reference :default "/Game/ThirdPerson/Input/Actions/IA_Lock.IA_Lock"))
  (bind _returnvalue (Game|GetPlayerCameraManager 0))
  (bind _player_bp (Variables|Default|GetPlayer%20BP))
  (bind _player_bp_2 (Variables|Default|GetPlayer%20BP))
  (bind _transformcomponent (Variables|/Script/Engine.PlayerCameraManager|GetTransformComponent _returnvalue))
  (bind _charactermovement (Variables|/Script/Engine.Character|GetCharacterMovement _player_bp))
  (bind _charactermovement_2 (Variables|/Script/Engine.Character|GetCharacterMovement _player_bp_2))
  (bind _returnvalue_2 (Transformation|GetWorldLocation _transformcomponent))
  ;[0 0.15 0.03167 0.5] Target Lock
  (:Started
    (Variables|Default|GetTarget%20lock%20actor
      (:then
        (Variables|Default|SetTarget%20lock%20actor 0) ; Disable target lock
        (Variables|/Script/Engine.CharacterMovementComponent|SetbOrientRotationToMovement _charactermovement true)
        (Variables|/Script/Engine.CharacterMovementComponent|SetbUseControllerDesiredRotation _charactermovement false)
        (Actor|DestroyActor (Variables|Default|GetTarget%20Lock%20Widget)) ; Destroy widget when player don't want to aim at enemies anymore
      )
      (:else
        (bind (_outhit _returnvalue_3) (Collision|SphereTraceForObjects "0, 0, 0" (+ (Math|Vector|MakeVector (.x _returnvalue_2) (.y _returnvalue_2) (+ (.z _returnvalue_2) 2e+01)) (* (Math|Vector|GetForwardVector (Transformation|GetWorldRotation _transformcomponent)) 1e+03)) 2e+02 (Utilities|Array|MakeArray "ObjectTypeQuery3") false 0 "ForDuration" true "(R=1.000000,G=0.000000,B=0.000000,A=1.000000)" "(R=0.000000,G=1.000000,B=0.000000,A=1.000000)" 2.0))
        (if _returnvalue_3
          (Variables|Default|SetTarget%20lock%20actor (.HitActor (Collision|BreakHitResult _outhit)))
          (Variables|/Script/Engine.CharacterMovementComponent|SetbOrientRotationToMovement _charactermovement_2 false)
          (Variables|/Script/Engine.CharacterMovementComponent|SetbUseControllerDesiredRotation _charactermovement_2 true)
          (bind _returnvalue_4 (Game|SpawnActorfromClass "/Game/Blueprint/BP_TargetLockWidget.BP_TargetLockWidget_C" (Math|Transform|MakeTransform (Math|Vector|MakeVector (.x (.location (Transformation|GetActorTransform (Variables|Default|GetTarget%20lock%20actor)))) (.y (.location (Transformation|GetActorTransform (Variables|Default|GetTarget%20lock%20actor)))) (+ (.z (.location (Transformation|GetActorTransform (Variables|Default|GetTarget%20lock%20actor)))) 2e+01)) (.rotation (Transformation|GetActorTransform (Variables|Default|GetTarget%20lock%20actor))) "1.000000,1.000000,1.000000") "AlwaysSpawn" "MultiplyWithRoot" 0 0))
          (bind _output_get (Variables|Default|SetTarget%20Lock%20Widget _returnvalue_4))
          (Transformation|AttachActorToActor _output_get (Variables|Default|GetTarget%20lock%20actor) "None" "SnapToTarget" "SnapToTarget" "SnapToTarget" true))))))

(event Input|EnhancedActionEvents|EnhancedInputActionIA_Attack
  (params (ActionValue :type Boolean) (ElapsedSeconds :type Float%20%28double-precision%29) (TriggeredSeconds :type Float%20%28double-precision%29) (InputAction :type Input%20Action%20Object%20Reference :default "/Game/ThirdPerson/Input/Actions/IA_Attack.IA_Attack"))
  (bind _player_bp (Variables|Default|GetPlayer%20BP))
  (bind _bpc_stats (Variables|/Game/ThirdPerson/Blueprints/BP_ThirdPersonCharacter_P1.BP_ThirdPersonCharacter_P1_C|GetBPC_Stats _player_bp))
  ;[0 0.02342 0.15 0.5] Sword Combo Animation
  (:Started
    (if (and (not (Variables|Default|GetIsAttacking?)) (>= (Variables|/Game/Blueprint/BPC_Stats.BPC_Stats_C|GetStamina (Variables|/Game/ThirdPerson/Blueprints/BP_ThirdPersonCharacter_P1.BP_ThirdPersonCharacter_P1_C|GetBPC_Stats (Variables|Default|GetPlayer%20BP))) 1e+01))
      (Variables|Default|SetIsAttacking? true)
      (Animation|Montage|PlayMontage (Variables|/Script/Engine.Character|GetMesh (Variables|Default|GetPlayer%20BP)) "/Game/Characters/Souls/Combat/SwordAttackCombo_Montage.SwordAttackCombo_Montage"
        (:then
          (Variables|/Game/Blueprint/BPC_Stats.BPC_Stats_C|SetregainStamina? _bpc_stats false)
          (Default|IncreaseValue _bpc_stats "NewEnumerator1" -1e+01 :!label _label))
        (:OnCompleted
          (Variables|Default|SetIsAttacking? false :!label _label_2)
          (Variables|Default|Setcombo? false)
          (Variables|/Game/Blueprint/BPC_Stats.BPC_Stats_C|SetregainStamina? (Variables|/Game/ThirdPerson/Blueprints/BP_ThirdPersonCharacter_P1.BP_ThirdPersonCharacter_P1_C|GetBPC_Stats (Variables|Default|GetPlayer%20BP)) true))
        (:OnInterrupted
          (goto _label_2))
        (:OnNotifyBegin
          (if (and (Variables|Default|GetIsAttacking?) (Variables|Default|Getcombo?))
            (Variables|Default|Setcombo? false)
            (goto _label)
            (else
              (Animation|Montage|MontageStop (Components|SkeletalMesh|GetAnimInstance (Variables|/Script/Engine.Character|GetMesh (Variables|Default|GetPlayer%20BP))) 0.2 "/Game/Characters/Souls/Combat/SwordAttackCombo_Montage.SwordAttackCombo_Montage")))))
      (else
        (Variables|Default|Setcombo? true)))))

(event Input|EnhancedActionEvents|EnhancedInputActionIA_Dodge
  (params (ActionValue :type Boolean) (ElapsedSeconds :type Float%20%28double-precision%29) (TriggeredSeconds :type Float%20%28double-precision%29) (InputAction :type Input%20Action%20Object%20Reference :default "/Game/ThirdPerson/Input/Actions/IA_Dodge.IA_Dodge"))
  (bind _player_bp (Variables|Default|GetPlayer%20BP))
  (bind _bpc_stats (Variables|/Game/ThirdPerson/Blueprints/BP_ThirdPersonCharacter_P1.BP_ThirdPersonCharacter_P1_C|GetBPC_Stats _player_bp))
  ;[0.15 0.15 0.15 0.5] Dodge logic in combat BPC
  (:Started
    (if (and (not (Variables|Default|GetIsDodging?)) (>= (Variables|/Game/Blueprint/BPC_Stats.BPC_Stats_C|GetStamina (Variables|/Game/ThirdPerson/Blueprints/BP_ThirdPersonCharacter_P1.BP_ThirdPersonCharacter_P1_C|GetBPC_Stats (Variables|Default|GetPlayer%20BP))) -25.0))
      (Variables|Default|SetIsDodging? true)
      (Utilities|FlowControl|Sequence
        (:then_0
          (if (Variables|/Script/Engine.CharacterMovementComponent|GetbUseControllerDesiredRotation (Variables|/Script/Engine.Character|GetCharacterMovement (Variables|Default|GetPlayer%20BP)))
            (switch string (Utilities|String|ToString(Text) (Class|KismetInputLibrary|KeyGetDisplayName (Variables|/Game/ThirdPerson/Blueprints/BP_ThirdPersonCharacter_P1.BP_ThirdPersonCharacter_P1_C|GetDirection%20Key (Variables|Default|GetPlayer%20BP)) true))
              (:W
                (Variables|Default|SetmovementDirection "NewEnumerator0"))
              (:A
                (Variables|Default|SetmovementDirection "NewEnumerator1"))
              (:S
                (Variables|Default|SetmovementDirection "NewEnumerator2"))
              (:D
                (Variables|Default|SetmovementDirection "NewEnumerator3")))
            (else
              (Variables|Default|SetmovementDirection "NewEnumerator0") ; If you are not using Staright movement is false
            )))
        (:then_1
          (Animation|Montage|PlayMontage (Variables|/Script/Engine.Character|GetMesh (Variables|Default|GetPlayer%20BP)) (Utilities|Select :Index (Variables|Default|GetmovementDirection) :NewEnumerator0 "/Game/Characters/Souls/Combat/Dodge/Dodge_F_Montage.Dodge_F_Montage" :NewEnumerator1 "/Game/Characters/Souls/Combat/Dodge/Dodge_L_Montage.Dodge_L_Montage" :NewEnumerator2 "/Game/Characters/Souls/Combat/Dodge/Dodge_B_Montage.Dodge_B_Montage" :NewEnumerator3 "/Game/Characters/Souls/Combat/Dodge/Dodge_R_Montage.Dodge_R_Montage")
            (:then
              (Variables|/Game/Blueprint/BPC_Stats.BPC_Stats_C|SetregainStamina? _bpc_stats false)
              (Default|IncreaseValue _bpc_stats "NewEnumerator1" -1e+01))
            (:OnCompleted
              (Variables|Default|SetIsDodging? false :!label _label)
              (Variables|/Game/Blueprint/BPC_Stats.BPC_Stats_C|SetregainStamina? (Variables|/Game/ThirdPerson/Blueprints/BP_ThirdPersonCharacter_P1.BP_ThirdPersonCharacter_P1_C|GetBPC_Stats (Variables|Default|GetPlayer%20BP)) true))
            (:OnInterrupted
              (goto _label))))))))

(event EventTick
  (params (DeltaSeconds :type Float%20%28single-precision%29))
  (bind _player_bp (Variables|Default|GetPlayer%20BP))
  (bind _target_lock_actor (Variables|Default|GetTarget%20lock%20actor))
  (bind _returnvalue (Transformation|GetActorLocation _player_bp))
  (bind _returnvalue_2 (Transformation|GetActorLocation _target_lock_actor))
  (bind _returnvalue_3 (Math|Rotator|FindLookatRotation _returnvalue _returnvalue_2))
  ;[0 0.15 0.03167 0.5] Target Lock
  ;;[0.0696 0.15 0 0.5] Target Lock Update
  (Variables|Default|GetTarget%20lock%20actor
    (:then
      (Pawn|SetControlRotation (Pawn|GetController (Variables|Default|GetPlayer%20BP)) (Math|Rotator|MakeRotator (.roll _returnvalue_3) (+ (.pitch _returnvalue_3) -2e+01) (.yaw _returnvalue_3))))
    (:else)))

(event EventBeginPlay
  ;[0.15 0 0 0.5] Get Player Class
  (bind _asbp_third_person_character (Utilities|Casting|CastToBP_ThirdPersonCharacter_P1 (Components|GetOwner)))
  (Variables|Default|SetPlayer%20BP _asbp_third_person_character))
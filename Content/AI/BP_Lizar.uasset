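; BP_Lizar is a melee enemy character, with boss options, that fights with montage-driven attacks and can be backstabbed.
; Damage feeds its stats component, linked to a widget health bar, and triggers camera shake, blood and sound.
; A looping timer runs sword sphere traces with a brief hit cooldown, while a boss secondary attack traces at one point.
; Death and backstab both end in ragdoll and delayed destruction.
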(event Custom|Damage%20Trace
  ;[0 0.009134 0.06125] Sword Traces
  (if (not (Variables|Default|GetIsDeath?))
    (bind (_outhit _returnvalue) (Collision|SphereTraceForObjects (Math|Vector|SelectVector (Variables|Default|GetBossStartSwordTracePos) (Transformation|GetWorldLocation (Variables|Default|GetStart%20sword%20trace%20arrow)) (Variables|Default|GetIsBoss?)) (Transformation|GetWorldLocation (Variables|Default|GetEnd%20sword%20trace%20arrow)) (Variables|Default|GetSwordAttackRadius) (Utilities|Array|MakeArray "ObjectTypeQuery3") false 0 "ForOneFrame"))
    (if _returnvalue
      (Utilities|FlowControl|DoOnce false :!label _label
        (:Completed
          (Game|Damage|ApplyDamage (.HitActor (Collision|BreakHitResult _outhit)) (Variables|Default|GetSword%20Damage) 0 0)
          (Utilities|FlowControl|Delay 0.3)
          (goto _label Reset))))))

(event EventPerfombackstab
  ;[0.15 0 0.006224 0.5] Die
  (Pawn|Components|CharacterMovement|DisableMovement (Variables|Character|GetCharacterMovement))
  (Animation|PlayAnimMontage "/Game/Characters/Souls/Combat/Stab_back/A_Stealthkillvictem_Montage.A_Stealthkillvictem_Montage" 1.0 "None")
  (Audio|PlaySound2D "/Game/Sound_Effect/Sword_Sound/Heroe_Sword_Hit_Quick/Heroe_Sword_Hit_Quick_6.Heroe_Sword_Hit_Quick_6" 1.0 1.0 0.0 0 0)
  (Utilities|FlowControl|Delay 2.0)
  (AddComponent|AddNiagaraComponent false)
  (Audio|PlaySound2D "/Game/Sound_Effect/Enemy_Hit/Enemy_die-1.Enemy_die-1" 1.0 1.0 0.0 0 0)
  (Variables|Default|SetIsDeath? true)
  (Physics|SetSimulatePhysics (Variables|Character|GetMesh) true)
  (AddComponent|AddNiagaraComponent false)
  (Utilities|FlowControl|Delay 2.0)
  (Actor|DestroyActor))

(event EventPointDamageTrace
  (bind _point_trace_pos (Variables|Default|GetPoint%20Trace%20Pos))
  (bind _returnvalue (Transformation|GetWorldLocation _point_trace_pos))
  ;[0.15 0.15 0.15 0.5] Boss secundary attack
  (bind (_outhit _returnvalue_2) (Collision|SphereTraceForObjects _returnvalue _returnvalue (Variables|Default|GetPointAttackRadius) (Utilities|Array|MakeArray "ObjectTypeQuery3") false 0 "ForDuration" true "(R=1.000000,G=0.000000,B=0.000000,A=1.000000)" "(R=0.000000,G=1.000000,B=0.000000,A=1.000000)" 2.0))
  (if _returnvalue_2
    (Game|Damage|ApplyDamage (.HitActor (Collision|BreakHitResult _outhit)) 3e+01 0 0)))

(event EventBeginSwordTrace
  ;[0 0.009134 0.06125] Sword Traces
  (Game|Feedback|ClientStartCameraShake (Game|GetPlayerController 0) "/Game/Blueprint/Camera_Shake_Combat/BP_Combat_Camera_Shake.BP_Combat_Camera_Shake_C" 1.0 "CameraLocal" "0, 0, 0") ; Every time you hit the enemy camera shake
  (bind _returnvalue (Utilities|Time|SetTimerbyEvent (delegate Custom|Damage%20Trace) 0.01 true)))

(event EventEndSwordTrace
  ;[0 0.009134 0.06125] Sword Traces
  (if (Utilities|Time|IsValidTimerHandle (stale EventBeginSwordTrace _returnvalue))
    (Utilities|Time|ClearandInvalidateTimerbyHandle (stale EventBeginSwordTrace _returnvalue))))

(event EventBeginPlay
  (bind _aswb_enemy_health (Utilities|Casting|CastToWB_Enemy_Health (UserInterface|GetWidget (Variables|Default|GetWidgetHealthBar))))
  (Variables|/Game/Blueprint/BPC_Stats.BPC_Stats_C|SetHealth%20Progress%20Bar (Variables|Default|GetBPC_Stats) (Variables|/Game/UI/HealthBar/WB_Enemy_Health.WB_Enemy_Health_C|GetHealth_Bar _aswb_enemy_health)))

(event Game|Damage|EventAnyDamage
  (params (Damage :type Float%20%28single-precision%29) (DamageType :type Damage%20Type%20Object%20Reference) (InstigatedBy :type Controller%20Object%20Reference) (DamageCauser :type Actor%20Object%20Reference))
  (Default|IncreaseValue (Variables|Default|GetBPC_Stats) "NewEnumerator0" (* Damage -1.0))
  (Game|Feedback|ClientStartCameraShake (Game|GetPlayerController 0) "/Game/Blueprint/Camera_Shake_Combat/BP_Combat_Camera_Shake.BP_Combat_Camera_Shake_C" 1.0 "CameraLocal" "0, 0, 0") ; Every time you hit the enemy camera shake
  (AddComponent|AddNiagaraComponent false) ; Blood VFX
  (Audio|PlaySound2D "/Game/Sound_Effect/Enemy_Hit/Enemy_Hit_Sound.Enemy_Hit_Sound" 1.0 1.0 0.0 0 0) ; Hit sound play
)

(event EventDie
  ;[0.15 0 0.006224 0.5] Die
  (Pawn|Components|CharacterMovement|DisableMovement (Variables|Character|GetCharacterMovement))
  (Utilities|FlowControl|DoOnce false
    (:Completed
      (Physics|SetSimulatePhysics (Variables|Character|GetMesh) true)
      (AddComponent|AddNiagaraComponent false)
      (Audio|PlaySound2D "/Game/Sound_Effect/Enemy_Hit/Enemy_hit_8.Enemy_hit_8" 1.0 1.0 0.0 0 0)
      (Variables|Default|SetIsDeath? true)
      (Utilities|FlowControl|Delay 3.0)
      (Actor|DestroyActor))))

(fn ConstructionScript)

(fn BigAttack
  (bind _returnvalue (Animation|PlayAnimMontage (Variables|Default|GetBigAttackMontage) 1.0 "None"))
  (return _returnvalue))

(fn Canbackstab
  (return true))

(fn RecoveringAttack1
  (bind _returnvalue (Animation|PlayAnimMontage (Variables|Default|GetStun_Montage) 1.0 "None"))
  (return _returnvalue))

(fn RoarBoss
  (return 0.0))

(fn SwordAttack
  (bind _returnvalue (Animation|PlayAnimMontage (Variables|Default|GetGhost_Heavy_Attack) 1.0 "None"))
  (return _returnvalue))

(fn SwordSecundaryAttack
  (bind _returnvalue (Animation|PlayAnimMontage (Variables|Default|GetGhost_Secundary_Attack) 1.0 "None"))
  (return _returnvalue))